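; Test flying character Blueprint for Reina that tunes a custom glide and shows movement debug info.
; CustomGlide toggles MoveUPScale, max fly speed and braking deceleration, zeroing the scale and raising speed while gliding.
; Two timelines, one for each state, drive MaxAcceleration over time after each toggle.
; Tick prints velocity, max fly speed and movement mode through DebugFormatter, which colors on-screen text by value type.
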(event Custom|Debug
  (bind _charactermovement (Variables|Character|GetCharacterMovement))
  (CallFunction|DebugFormatter "NewEnumerator4" "Velocity" (Utilities|String|ToString(Float) (Math|Vector|VectorLength (Transformation|GetVelocity))))
  (CallFunction|DebugFormatter "NewEnumerator4" "Max fly speed" (Utilities|String|ToString(Float) (Variables|/Script/Engine.CharacterMovementComponent|GetMaxFlySpeed _charactermovement)))
  (CallFunction|DebugFormatter "NewEnumerator8" "Velocity" (Utilities|String|EnumtoString (Variables|/Script/Engine.CharacterMovementComponent|GetMovementMode _charactermovement))))

(event EventTick
  (params (DeltaSeconds :type Float%20%28single-precision%29))
  (CallFunction|Debug))

(event EventCustomGlide
  (params (bIsEnabled :type Boolean))
  (bind _charactermovement (Variables|Character|GetCharacterMovement))
  (Audio|Components|Audio|Stop (Variables|Default|GetAcceleration))
  (if bIsEnabled
    (Variables|Default|SetMoveUPScale 0.0)
    (Variables|/Script/Engine.CharacterMovementComponent|SetMaxFlySpeed _charactermovement 1e+04) ; 飛行速度
    (Variables|/Script/Engine.CharacterMovementComponent|SetBrakingDecelerationFlying _charactermovement 5e+02) ; 減速度
    (bind _value (Timeline|Acceleration PlayFromStart)
      (:Update
        (Variables|/Script/Engine.CharacterMovementComponent|SetMaxAcceleration _charactermovement _value) ; 加速度
      ))
    (else
      (Variables|Default|SetMoveUPScale 1.0)
      (Variables|/Script/Engine.CharacterMovementComponent|SetMaxFlySpeed _charactermovement 1.2e+03)
      (Variables|/Script/Engine.CharacterMovementComponent|SetBrakingDecelerationFlying _charactermovement 1e+03)
      (bind _value_2 (Timeline|ReAcceleration PlayFromStart)
        (:Update
          (Variables|/Script/Engine.CharacterMovementComponent|SetMaxAcceleration _charactermovement _value_2))))))

(event EventBeginPlay)

(fn ConstructionScript
  (|CallParentFunction))

(fn DebugFormatter
  (params (colorMode :type EDebugType%20Enum :default "NewEnumerator0") (title :type String) (value :type String))
  (bind _returnvalue (Utilities|String|Append title " = " value))
  (switch Utilities|FlowControl|Switch|SwitchonEDebugType colorMode
    (:NewEnumerator0
      (Development|PrintString _returnvalue true false "(R=0.401042,G=0.000000,B=0.002201,A=1.000000)" 0.0))
    (:NewEnumerator1
      (Development|PrintString _returnvalue true false "(R=0.463542,G=0.050700,B=0.359655,A=1.000000)" 0.0))
    (:NewEnumerator3
      (Development|PrintString _returnvalue true false "(R=0.000000,G=0.340637,B=1.000000,A=1.000000)" 0.0))
    (:NewEnumerator4
      (Development|PrintString _returnvalue true false "(R=0.086847,G=0.463542,B=0.000000,A=1.000000)" 0.0))
    (:NewEnumerator5
      (Development|PrintString _returnvalue true false "(R=0.000000,G=0.340637,B=1.000000,A=1.000000)" 0.0))
    (:NewEnumerator6
      (Development|PrintString _returnvalue true false "(R=0.000000,G=0.340637,B=1.000000,A=1.000000)" 0.0))
    (:NewEnumerator7
      (Development|PrintString _returnvalue true false "(R=1.000000,G=0.120101,B=0.000000,A=1.000000)" 0.0))
    (:NewEnumerator8
      (Development|PrintString _returnvalue true false "(R=0.000000,G=0.192708,B=0.113557,A=1.000000)" 0.0))))